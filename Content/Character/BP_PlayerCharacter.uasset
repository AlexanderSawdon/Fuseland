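; Player character for top-down play that moves on world axes and turns its mesh to face the mouse cursor.
; BeginPlay adds the top-down Enhanced Input mapping context and shows the cursor.
; Each tick intersects the deprojected cursor ray with the world Z=0 plane, yaws the mesh toward that point and marks it with a debug sphere.
; Shooting is a placeholder that only draws a debug sphere.
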(event `EnhancedInput|/Game/Input/Actions/IA_MouseOne`
  (params (ActionValue :type Boolean) (ElapsedSeconds :type "Float (double-precision)") (TriggeredSeconds :type "Float (double-precision)") (InputAction :type "InputAction Object Reference" :default "/Game/Input/Actions/IA_MouseOne.IA_MouseOne"))
  ;[1 1 1] Shoot
  (:`Triggered`
    (`KismetSystemLibrary.DrawDebugSphere` (0.0 0.0 0.0))))

(event `self.ReceiveBeginPlay`
  ;[1 1 1] Cast Controller
  (bind _asplayer_controller (cast `PlayerController` (`self.GetController`)))
  (`EnhancedInputSubsystemInterface.AddMappingContext` (pcsubsystem `EnhancedInputLocalPlayerSubsystem` _asplayer_controller) "/Game/Input/IMC_TopDown.IMC_TopDown" 0 (struct))
  (set `PlayerController.bShowMouseCursor` true (`GameplayStatics.GetPlayerController` 0)))

(event `EnhancedInput|/Game/Input/Actions/IA_Move`
  (params (ActionValue :type "Vector2D Structure") (ElapsedSeconds :type "Float (double-precision)") (TriggeredSeconds :type "Float (double-precision)") (InputAction :type "InputAction Object Reference" :default "/Game/Input/Actions/IA_Move.IA_Move"))
  ;[1 1 1] Movement
  (:`Triggered`
    (`self.AddMovementInput` (1.0 0.0 0.0) ActionValue_X)
    (`self.AddMovementInput` (0.0 1.0 0.0) ActionValue_Y)))

(event `self.ReceiveTick`
  (params (DeltaSeconds :type "Float (single-precision)"))
  (bind (_returnvalue_roll _returnvalue_pitch) (`KismetMathLibrary.BreakRotator` (`self.K2_GetActorRotation`)))
  (bind _returnvalue (`KismetMathLibrary.Vector_Up`))
  (bind (_worldlocation _worlddirection) (`PlayerController.DeprojectMousePositionToWorld` (`GameplayStatics.GetPlayerController` 0)))
  (bind _returnvalue_2 (+ _worldlocation (* _worlddirection (/ (`KismetMathLibrary.Dot_VectorVector` (- (`KismetMathLibrary.Vector_Zero`) _worldlocation) _returnvalue) (`KismetMathLibrary.Dot_VectorVector` _worlddirection _returnvalue)))))
  (bind (_returnvalue_roll_2 _returnvalue_pitch_2 _returnvalue_yaw) (`KismetMathLibrary.BreakRotator` (`KismetMathLibrary.FindLookAtRotation` (`self.K2_GetActorLocation`) _returnvalue_2)))
  ;[1 1 1] Rotate Player
  (`SceneComponent.K2_SetWorldRotation` (`self.PlayerMesh`) (`KismetMathLibrary.MakeRotator` _returnvalue_roll _returnvalue_pitch _returnvalue_yaw) false true)
  (`KismetSystemLibrary.DrawDebugSphere` _returnvalue_2 10.0 12 (struct :`R` 1.0 :`B` 0.159153 :`A` 1.0) 0.0 1.0))

(fn `UserConstructionScript`)